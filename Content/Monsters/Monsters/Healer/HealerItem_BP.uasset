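; HealerItem_BP is the Healer monster's item actor, a short-lived visual for a help action, with no healing logic of its own.
; BeginPlay disables actor collision, and Tick grows MonsterItem exponentially by a fixed per-frame factor, so growth depends on frame rate.
; MonsterHelp nudges the item upward and attaches a heal aura, then after timed delays adds a resurrection effect, hides the item and destroys the actor.
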(event `self.ReceiveBeginPlay`
  (`self.SetActorEnableCollision` false))

(event `self.ReceiveTick`
  (params (DeltaSeconds :type "Float (single-precision)"))
  (bind _monsteritem (`self.MonsterItem`))
  (`SceneComponent.SetWorldScale3D` _monsteritem (* (`SceneComponent.K2_GetComponentScale` _monsteritem) 1.005)))

(event `self.MonsterHelp`
  (params (`I am Todd` :type "/Game/Monsters/Todd/BP_Todd Object Reference"))
  (bind _monsteritem (`self.MonsterItem`))
  (`PrimitiveComponent.AddImpulse` _monsteritem (0.0 0.0 50.0) "None" false)
  (`GameplayStatics.SpawnEmitterAttached` "/Game/InfinityBladeEffects/Effects/FX_Ability/Heal/P_Heal_Aura.P_Heal_Aura" _monsteritem)
  (`KismetSystemLibrary.Delay` 1.5)
  (`GameplayStatics.SpawnEmitterAttached` "/Game/InfinityBladeEffects/Effects/FX_Cines/Ausar/P_Ausar_Resurrection.P_Ausar_Resurrection" _monsteritem)
  (`KismetSystemLibrary.Delay` 3.0)
  (`SceneComponent.SetVisibility` (`self.MonsterItem`) false false)
  (`KismetSystemLibrary.Delay` 1.0)
  (`self.K2_DestroyActor`))

(fn `UserConstructionScript`
  (`parent.UserConstructionScript`))