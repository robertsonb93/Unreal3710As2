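; FlightItem_BP is an item that grants a monster temporary flight through its MonsterHelp event.
; On BeginPlay it disables its collision and sets itself to expire one second after the LifeSpan duration.
; MonsterHelp adds a scene component to the target as the projectile's homing target, then enables CanFly and Flying movement.
; After a LifeSpan delay it clears CanFly and restores Walking.
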(event `self.ReceiveBeginPlay`
  (`PrimitiveComponent.SetCollisionEnabled` (`self.Collision`) "NoCollision")
  (`self.SetLifeSpan` (`KismetMathLibrary.Conv_IntToDouble` (+ (`self.LifeSpan`) 1))))

(event `self.MonsterHelp`
  (params (`I am Todd` :type "/Game/Monsters/Todd/BP_Todd Object Reference"))
  (bind _returnvalue (`AddComponent|NODE_AddSceneComponent-0` :`self` `I am Todd`))
  (set `ProjectileMovementComponent.HomingTargetComponent` _returnvalue (`self.ProjectileMovement`))
  (`CharacterMovementComponent.SetMovementMode` (`Character.CharacterMovement` `I am Todd`) "MOVE_Flying" 0)
  (set `/Game/Monsters/Todd/BP_Todd.CanFly` true `I am Todd`)
  (`KismetSystemLibrary.Delay` (`KismetMathLibrary.Conv_IntToDouble` (`self.LifeSpan`)))
  (set `/Game/Monsters/Todd/BP_Todd.CanFly` false `I am Todd`)
  (`CharacterMovementComponent.SetMovementMode` (`Character.CharacterMovement` `I am Todd`) "MOVE_Walking" 0))

(fn `UserConstructionScript`
  (`parent.UserConstructionScript`))