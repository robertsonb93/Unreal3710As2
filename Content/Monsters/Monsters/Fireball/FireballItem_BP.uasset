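; Fireball item Blueprint for a projectile that plays a launch sound, trails fire from its MonsterItem component and lives two seconds.
; A hit plays an attack sound and destroys it early.
; Any destruction, by hit or timeout, spawns an explosion whose particle bounds size a class trace and radial damage.
; The trace's Friends are spared, and damage is credited to the first player's controller.
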(event `self.ReceiveBeginPlay`
  (`GameplayStatics.PlaySound2D` "/Game/Sound/pewpew.pewpew")
  (`self.SetLifeSpan` 2.0)
  (`GameplayStatics.SpawnEmitterAttached` "/Game/InfinityBladeEffects/Effects/FX_Monsters/FX_Monster_SpiderBoss/Fire/P_TailFire.P_TailFire" (`self.MonsterItem`)))

(event `self.ReceiveHit`
  (params (MyComp :type "PrimitiveComponent Object Reference") (Other :type "Actor Object Reference") (OtherComp :type "PrimitiveComponent Object Reference") (bSelfMoved :type Boolean) (HitLocation :type "Vector Structure") (HitNormal :type "Vector Structure") (NormalImpulse :type "Vector Structure") (Hit :type "HitResult Structure (by ref)"))
  (`GameplayStatics.PlaySound2D` "/Game/Sound/fireattack.fireattack")
  (`self.K2_DestroyActor`))

(event `self.ReceiveDestroyed`
  (bind _returnvalue (`GameplayStatics.SpawnEmitterAtLocation` "/Game/StarterContent/Particles/P_Explosion.P_Explosion" (`SceneComponent.K2_GetComponentLocation` (`self.MonsterItem`))))
  (bind (_origin _boxextent _sphereradius) (`KismetSystemLibrary.GetComponentBounds` _returnvalue))
  (bind _friends (`self.TraceForActorClasses` _sphereradius _origin (+ _origin _boxextent)))
  (`GameplayStatics.ApplyRadialDamage` 100.0 _origin _sphereradius null _friends self (`GameplayStatics.GetPlayerController` 0)))

(fn `UserConstructionScript`
  (`parent.UserConstructionScript`))