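; Monster_Base_BP is a base monster Blueprint that disappears when BP_Todd overlaps it and returns through its checkpoint.
; On overlap it hides the root and its children and disables collision instead of destroying the actor.
; On BeginPlay it binds Respawn to MyCheckpoint's respawn-world event, or prints a warning if none is set.
; Respawn restores collision and root visibility, without propagating visibility to children.
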(event `self.ReceiveActorBeginOverlap`
  (params (OtherActor :type "Actor Object Reference"))
  (cast `/Game/Monsters/Todd/BP_Todd` OtherActor)
  (`SceneComponent.SetVisibility` (`self.DefaultSceneRoot`) false true)
  (`self.SetActorEnableCollision` false))

(event `self.ReceiveBeginPlay`
  (bind _mycheckpoint (`self.MyCheckpoint`))
  (`/Engine/EditorBlueprintResources/StandardMacros.IsValid` _mycheckpoint
    (:`Is Valid`
      (add `/Game/Monsters/Monsters/Checkpoint/CheckPoint.RespawnWorld` _mycheckpoint (delegate `Respawn`)))
    (:`Is Not Valid`
      (`KismetSystemLibrary.PrintString` (`KismetStringLibrary.Concat_StrStr` (`KismetSystemLibrary.GetObjectName` self) "Has Invalid Checkpoint, Ensure It has a checkpoint set")))))

(event `Respawn`
  (`SceneComponent.SetVisibility` (`self.DefaultSceneRoot`) true false)
  (`self.SetActorEnableCollision` true))

(fn `UserConstructionScript`)