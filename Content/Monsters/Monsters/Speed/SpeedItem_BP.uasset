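; SpeedItem_BP is a monster item that gives the Todd character a temporary sprint boost.
; It plays a sound and disables its collision on spawn, then on MonsterHelp teleports beside Todd and attaches to him.
; It raises his max walk speed with an attached aura particle, then after a short delay restores the saved speed and destroys itself in a burst of sparks.
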(event `self.ReceiveBeginPlay`
  (`GameplayStatics.PlaySound2D` "/Game/Sound/sprint.sprint" 10.0)
  (`self.SetActorEnableCollision` false))

(event `self.MonsterHelp`
  (params (`I am Todd` :type "/Game/Monsters/Todd/BP_Todd Object Reference"))
  (bind _charactermovement (`Character.CharacterMovement` `I am Todd`))
  (`self.K2_SetActorLocation` (+ (* (`SceneComponent.GetRightVector` (`Character.Mesh` `I am Todd`)) -50) (`self.K2_GetActorLocation` `I am Todd`)) false true)
  (`self.K2_AttachToActor` `I am Todd` "None" "KeepWorld" "KeepWorld" "KeepWorld" false)
  (set `self.DefaultWalkSpeed` (`CharacterMovementComponent.MaxWalkSpeed` _charactermovement))
  ;[1 1 1] We ramp up todds max speed, add a particle for some Fx, wait for a few seconds then destroy the componene and set his speed back to original
  (set `CharacterMovementComponent.MaxWalkSpeed` 1200.0 _charactermovement)
  (bind _returnvalue (`GameplayStatics.SpawnEmitterAttached` "/Game/InfinityBladeEffects/Effects/FX_Archive/P_AttackPower_Aura.P_AttackPower_Aura" (`Character.Mesh` `I am Todd`)))
  (`KismetSystemLibrary.Delay` 2.0)
  (`ActorComponent.K2_DestroyComponent` _returnvalue)
  (set `CharacterMovementComponent.MaxWalkSpeed` (`self.DefaultWalkSpeed`) (`Character.CharacterMovement` `I am Todd`))
  (`self.K2_DestroyActor`))

(event `self.ReceiveDestroyed`
  (`GameplayStatics.SpawnEmitterAtLocation` "/Game/InfinityBladeEffects/Effects/FX_Monsters/FX_Monster_Ausar/P_AU_Taunt_sparks.P_AU_Taunt_sparks" (`SceneComponent.K2_GetComponentLocation` (`self.MonsterItem`))))

(fn `UserConstructionScript`
  (`parent.UserConstructionScript`))