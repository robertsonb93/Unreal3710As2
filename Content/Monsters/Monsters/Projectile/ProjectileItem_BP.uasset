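; Monster projectile item that charges up with fire effects and bursts when destroyed.
; BeginPlay attaches a charge-up emitter to MonsterItem, adds rotating movement and sets a short lifespan, while Tick grows MonsterItem's scale by a fixed, frame-rate-dependent step.
; Destroyed spawns fire aura and explosion flare emitters at the item's location, with aura cleanup placed behind a Delay on the actor being destroyed.
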(event `self.ReceiveBeginPlay`
  (`GameplayStatics.SpawnEmitterAttached` "/Game/InfinityBladeEffects/Effects/FX_Mobile/Fire/combat/P_Circle_ChargeUp_Fire_Phase2.P_Circle_ChargeUp_Fire_Phase2" (`self.MonsterItem`))
  (`self.SetLifeSpan` 5.0)
  (`AddComponent|NODE_AddRotatingMovementComponent-0`))

(event `self.ReceiveTick`
  (params (DeltaSeconds :type "Float (single-precision)"))
  (bind _monsteritem (`self.MonsterItem`))
  (`SceneComponent.SetWorldScale3D` _monsteritem (+ (`SceneComponent.K2_GetComponentScale` _monsteritem) (0.01 0.01 0.01))))

(event `self.ReceiveDestroyed`
  (bind _returnvalue (`SceneComponent.K2_GetComponentLocation` (`self.MonsterItem`)))
  (bind _returnvalue_2 (`GameplayStatics.SpawnEmitterAtLocation` "/Game/InfinityBladeEffects/Effects/FX_Mobile/Fire/combat/P_AuraCircle_Fire_02.P_AuraCircle_Fire_02" _returnvalue))
  (`GameplayStatics.SpawnEmitterAtLocation` "/Game/InfinityBladeEffects/Effects/FX_Cines/cinema03/P_CIN_IB_Explosion_Flare.P_CIN_IB_Explosion_Flare" _returnvalue)
  (`KismetSystemLibrary.Delay` 4.0)
  (`SceneComponent.SetVisibility` _returnvalue_2 false false)
  (`ActorComponent.K2_DestroyComponent` _returnvalue_2))

(fn `UserConstructionScript`
  (`parent.UserConstructionScript`))