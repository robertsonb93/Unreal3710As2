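; BP_OwlProjectile is the owl monster's projectile, which damages BP_Todd on impact.
; On a hit against Todd, it subtracts the Sphere component's current speed, rounded up, from his Health, clamped to a valid range, and spawns a blood splatter at the hit location.
; Any hit, on Todd or otherwise, leads to the actor destroying itself after a short delay.
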(event `self.ReceiveHit`
  (params (MyComp :type "PrimitiveComponent Object Reference") (Other :type "Actor Object Reference") (OtherComp :type "PrimitiveComponent Object Reference") (bSelfMoved :type Boolean) (HitLocation :type "Vector Structure") (HitNormal :type "Vector Structure") (NormalImpulse :type "Vector Structure") (Hit :type "HitResult Structure (by ref)"))
  (bind _asbp_todd (cast `/Game/Monsters/Todd/BP_Todd` Other)
    (:`then`
      (set `/Game/Monsters/Todd/BP_Todd.Health` (`KismetMathLibrary.Clamp` (- (`/Game/Monsters/Todd/BP_Todd.Health` _asbp_todd) (`KismetMathLibrary.FCeil` (`KismetMathLibrary.VSize` (`SceneComponent.GetComponentVelocity` (`self.Sphere`))))) 0 100) _asbp_todd)
      (`GameplayStatics.SpawnEmitterAtLocation` "/Game/Monsters/Owls/Meat/P_BloodSplatter.P_BloodSplatter" HitLocation))
    (:`CastFailed`
      _))
  (`KismetSystemLibrary.Delay` 1.0)
  (`self.K2_DestroyActor`))

(fn `UserConstructionScript`)