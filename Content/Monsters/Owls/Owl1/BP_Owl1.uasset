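; Owl monster Blueprint with a destructible mesh that loses health when hit, scaled by the striking component's speed.
; On death it enables cap physics, reveals and launches the splatterer (tombstone), and fractures the mesh with heavy damage and an opposing impulse.
; Fracturing triggers blood particles, then delayed removal of mesh and cap.
; Attack only spawns an explosion effect, and Move is an empty stub.
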(event `self.Owl1_Owl1_DM.OnComponentHit`
  (params (HitComponent :type "PrimitiveComponent Object Reference") (OtherActor :type "Actor Object Reference") (OtherComp :type "PrimitiveComponent Object Reference") (NormalImpulse :type "Vector Structure") (Hit :type "HitResult Structure (by ref)"))
  ;[1 1 1] Handles The life system for the owls, takes damage when the destructible mesh is hit by objects, and the amount of damage is a based on the speed it was hit
  (bind _output_get (set `self.Health` (- (`self.Health`) (* (`KismetMathLibrary.VSize` (`SceneComponent.GetComponentVelocity` OtherComp)) 0.01))))
  (if (>= _output_get 0.01)
    (`KismetSystemLibrary.PrintString` (`KismetStringLibrary.Concat_StrStr` (`KismetStringLibrary.Conv_DoubleToString` _output_get) " Current Owl Health"))
    (else
      (`self.DeathEvent`))))

(event `DeathEvent`
  (bind _tombstone_vector (`self.Tombstone Vector`))
  (bind _owl1_owl1_dm (`self.Owl1_Owl1_DM`))
  (bind _returnvalue (`KismetMathLibrary.NegateVector` _tombstone_vector))
  ;[1 1 1] Is called when the owls health reaches zero, basically activates the tombstone and damages the DM
  (set `self.IsAlive` false)
  (`PrimitiveComponent.SetSimulatePhysics` (`self.Owl1_Cap`) true)
  (`SceneComponent.SetVisibility` (`self.owl_splatterer`) true false)
  (`PrimitiveComponent.SetSimulatePhysics` (`self.owl_splatterer`) true)
  (`PrimitiveComponent.SetAllPhysicsLinearVelocity` (`self.owl_splatterer`) _tombstone_vector true)
  (`DestructibleComponent.ApplyDamage` _owl1_owl1_dm 10000.0 (`SceneComponent.K2_GetComponentLocation` _owl1_owl1_dm) _returnvalue (`KismetMathLibrary.VSize` _returnvalue)))

(event `self.ReceiveBeginPlay`
  ;[1 1 1] Everyone likes a good blood Splatter
  (add `DestructibleComponent.OnComponentFracture` (`self.Owl1_Owl1_DM`) (delegate `BloodParticles`)))

(event `BloodParticles`
  (params (HitPoint :type "Vector Structure (by ref)") (HitDirection :type "Vector Structure (by ref)"))
  ;[1 1 1] Everyone likes a good blood Splatter
  (`GameplayStatics.SpawnEmitterAttached` "/Game/Monsters/Owls/Meat/P_BloodSplatter.P_BloodSplatter" (`self.Owl1_Owl1_DM`) "None" (0.0 0.0 0.0) (struct) "SnapToTarget")
  (`KismetSystemLibrary.Delay` 15.0)
  (`ActorComponent.K2_DestroyComponent` (`self.Owl1_Owl1_DM`))
  (`ActorComponent.K2_DestroyComponent` (`self.Owl1_Cap`)))

(event `Attack`
  (`GameplayStatics.SpawnEmitterAtLocation` "/Game/StarterContent/Particles/P_Explosion.P_Explosion" (`self.K2_GetActorLocation` self)))

(event `Move`
  (params (Destination :type "Vector Structure")))

(fn `UserConstructionScript`)