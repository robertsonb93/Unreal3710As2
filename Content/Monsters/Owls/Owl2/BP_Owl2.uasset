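; Flying owl monster character that moves along a set direction, launches BP_OwlProjectile attacks and can be killed by damage.
; Tick drives movement input, with a once-per-second downward trace meant to nudge it into a height band.
; Damage from anything but owl projectiles drains health; death restores gravity and swaps the mesh for a destructible plus physics splatterer.
; Fracture spawns blood, then delayed cleanup destroys the actor.
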(event `self.ReceiveAnyDamage`
  (params (Damage :type "Float (single-precision)") (DamageType :type "DamageType Object Reference") (InstigatedBy :type "Controller Object Reference") (DamageCauser :type "Actor Object Reference"))
  ;[1 1 1] Handles The life system for the owls, takes damage when the destructible mesh is hit by objects, and the amount of damage is a based on the speed it was hit
  (cast `/Game/Monsters/Owls/BP_OwlProjectile` DamageCauser
    (:`CastFailed`
      (bind _output_get (set `self.Health` (- (`self.Health`) Damage)))
      (if (not (>= _output_get 0.01))
        (`self.DeathEvent`)))))

(event `DeathEvent`
  (bind _tombstone_vector (`self.Tombstone Vector`))
  (bind _returnvalue (`KismetMathLibrary.NegateVector` _tombstone_vector))
  ;[1 1 1] Is called when the owls health reaches zero, basically activates the tombstone and damages the DM
  (set `self.IsAlive` false)
  (`SceneComponent.SetVisibility` (`self.owl_splatterer`) true false)
  (`PrimitiveComponent.SetSimulatePhysics` (`self.owl_splatterer`) true)
  (`PrimitiveComponent.SetAllPhysicsLinearVelocity` (`self.owl_splatterer`) _tombstone_vector true)
  (`DestructibleComponent.ApplyDamage` (`self.Owl2_Object001_DM`) 9000000.0 (`self.K2_GetActorLocation`) _returnvalue (`KismetMathLibrary.VSize` _returnvalue))
  (`SceneComponent.SetVisibility` (`self.Mesh`) false false)
  (`SceneComponent.SetVisibility` (`self.Owl2_Object001_DM`) true false)
  (`PrimitiveComponent.SetEnableGravity` (`self.CapsuleComponent`) true)
  (`PrimitiveComponent.SetEnableGravity` (`self.Mesh`) true)
  (`PrimitiveComponent.SetEnableGravity` (`self.Owl2_Object001_DM`) true)
  (`PrimitiveComponent.SetEnableGravity` (`self.owl_splatterer`) true)
  ;[1 1 1] Supposedly there is a bug with Disabling Gravity on a skeletal mesh, so we instead turned the scale of it down in teh constructor
  (set `CharacterMovementComponent.GravityScale` 3.0 (`self.CharacterMovement`)))

(event `self.Owl2_Object001_DM.OnComponentFracture`
  (params (HitPoint :type "Vector Structure (by ref)") (HitDirection :type "Vector Structure (by ref)"))
  ;[1 1 1] Everyone likes a good blood Splatter
  (`GameplayStatics.SpawnEmitterAttached` "/Game/Monsters/Owls/Meat/P_BloodSplatter.P_BloodSplatter" (`self.Owl2_Object001_DM`) "None" (0.0 0.0 0.0) (struct) "SnapToTarget")
  ;;[1 1 1] Kill the actor
  (`KismetSystemLibrary.Delay` 15.0)
  (`ActorComponent.K2_DestroyComponent` (`self.Owl2_Object001_DM`))
  (`KismetSystemLibrary.Delay` 15.0)
  (`self.K2_DestroyActor`))

(event `self.ReceiveTick`
  (params (DeltaSeconds :type "Float (single-precision)"))
  (bind _destinationdirection (`self.DestinationDirection`))
  ;[1 1 1] Calculate our next motion
  (set `self.DeltaSecs` (+ (`self.DeltaSecs`) DeltaSeconds))
  (if (`self.IsAlive`)
    (if (>= (`self.DeltaSecs`) 1.0)
      (bind _destdirmodified (`self.HeightCheck` _destinationdirection))
      (set `self.DeltaSecs` 0.0)
      (`self.AddMovementInput` _destdirmodified)
      (else
        (`self.AddMovementInput` _destinationdirection)))))

(event `Move`
  (params (Destination :type "Vector Structure"))
  ;[1 1 1] Sets a move to direction, the actual moving is handle with ticks
  (set `self.DestinationDirection` (`KismetMathLibrary.Normal` (- Destination (`self.K2_GetActorLocation`)))))

(event `Attack`
  (params (TargetLocation :type "Vector Structure"))
  ;[1 1 1] Called When we are going to launch an attack
  (bind _returnvalue (`|SpawnActorFromClass` "/Game/Monsters/Owls/BP_OwlProjectile.BP_OwlProjectile_C" (`KismetMathLibrary.MakeTransform` (+ (* (`self.GetActorUpVector`) -50) (`self.K2_GetActorLocation`)) (`self.K2_GetActorRotation`) (`self.GetActorScale3D`)) "AdjustIfPossibleButAlwaysSpawn" "OverrideRootScale" null self))
  (`PrimitiveComponent.SetAllPhysicsLinearVelocity` (`/Game/Monsters/Owls/BP_OwlProjectile.Sphere` _returnvalue) (- (`self.K2_GetActorLocation`) TargetLocation) false))

(fn `HeightCheck`
  (params (DestinationDirection :type "Vector Structure"))
  (returns (DestDirModified :type "Vector Structure"))
  (bind _returnvalue (`self.K2_GetActorLocation`))
  (bind _outhit (`KismetSystemLibrary.LineTraceSingleForObjects` :`Start` _returnvalue :`End` (- _returnvalue (0.0 0.0 10000.0)) :`ObjectTypes` (`|MakeArray` "ObjectTypeQuery1" :!type "EObjectTypeQuery Enum") :`DrawDebugType` "ForDuration"))
  (bind (_bblockinghit _binitialoverlap _time _location _impactpoint _normal _impactnormal _physmat _hitactor _hitcomponent _hitbonename _hititem _faceindex _tracestart _traceend) (`GameplayStatics.BreakHitResult` _outhit))
  (bind _returnvalue_2 (`KismetMathLibrary.Abs` (.z (- _tracestart _traceend))))
  (if (<= (`self.MinHeight`) _returnvalue_2)
    (if (>= (`self.MaxHeight`) _returnvalue_2)
      (set `self.ZChoice` (.z DestinationDirection))
      (else
        (set `self.ZChoice` -10.0)))
    (else
      (set `self.ZChoice` 10.0)))
  (return (`KismetMathLibrary.MakeVector` (.x DestinationDirection) (.y DestinationDirection) (`self.ZChoice`))))

(fn `UserConstructionScript`
  (set `CharacterMovementComponent.GravityScale` 0.0 (`self.CharacterMovement`)))