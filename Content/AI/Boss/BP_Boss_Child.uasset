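; BP_Boss_Child is a child boss Blueprint that flies between two stored positions, Hi and Lo.
; BeginPlay flags it as flying and sets Destination to its current location.
; Every Tick it adds movement input toward Destination, with no arrival check.
; Each Move event call uses a FlipFlop to switch Destination between Hi and Lo, ignoring the event's own Destination input.
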(event `self.ReceiveTick`
  (params (DeltaSeconds :type "Float (single-precision)"))
  (`self.AddMovementInput` (`KismetMathLibrary.GetDirectionUnitVector` (`self.K2_GetActorLocation`) (`self.Destination`))))

(event `Move`
  (params (Destination :type "Vector Structure"))
  (`/Engine/EditorBlueprintResources/StandardMacros.FlipFlop`
    (:`A`
      (set `self.Destination` (`self.Hi`)))
    (:`B`
      (set `self.Destination` (`self.Lo`)))))

(event `self.ReceiveBeginPlay`
  ;[1 1 1] Comment
  (set `self.IsFlying` true)
  (set `self.Destination` (`self.K2_GetActorLocation`)))

(fn `UserConstructionScript`
  (`parent.UserConstructionScript`))