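; Boss character that exposes movement, jump and three attack events, with no decision logic of its own.
; Move uses AIMoveTo, and Jump is gated by IsLanded, refreshed every tick by a short downward line trace from the mesh.
; Melee damages BP_Todd actors overlapping a sphere, while mid and long range attacks spawn their attack actors just in front of the boss.
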(event `self.ReceiveActorBeginOverlap`
  (params (OtherActor :type "Actor Object Reference")))

(event `self.ReceiveTick`
  (params (DeltaSeconds :type "Float (single-precision)"))
  (`self.LandedFunc`))

(event `JumpEvent`
  (if (`self.IsLanded`)
    (`self.Jump`)))

(event `Move`
  (params (Destination :type "Vector Structure"))
  (`|AIMoveTo` self Destination))

(event `Melee`
  (for _array_element (`PrimitiveComponent.GetOverlappingActors` (`self.Sphere`) "/Game/Monsters/Todd/BP_Todd.BP_Todd_C")
    (`GameplayStatics.ApplyDamage` _array_element 15.0)))

(event `MidRangeAttack`
  (`|SpawnActorFromClass` "/Game/AI/Boss/MidRangeAttack.MidRangeAttack_C" (`KismetMathLibrary.MakeTransform` (+ (* (`SceneComponent.GetForwardVector` (`self.Mesh`)) 15) (`self.K2_GetActorLocation`)) (`self.K2_GetActorRotation`)) "Undefined" "OverrideRootScale" null null))

(event `LongRangeAttack`
  (`|SpawnActorFromClass` "/Game/AI/Boss/LongRangeAttack.LongRangeAttack_C" (`KismetMathLibrary.MakeTransform` (+ (* (`SceneComponent.GetForwardVector` (`self.Mesh`)) 15) (`self.K2_GetActorLocation`)) (`self.K2_GetActorRotation`)) "Undefined" "OverrideRootScale" null null))

(fn `LandedFunc`
  (bind _mesh (`self.Mesh`))
  (bind _returnvalue (`SceneComponent.K2_GetComponentLocation` _mesh))
  (bind (_outhit _returnvalue_2) (`KismetSystemLibrary.LineTraceSingle` _returnvalue (+ _returnvalue (* (`SceneComponent.GetUpVector` _mesh) -5)) "TraceTypeQuery1"))
  (set `self.IsLanded` _returnvalue_2))

(fn `UserConstructionScript`)