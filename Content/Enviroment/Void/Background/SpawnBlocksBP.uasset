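; SpawnBlocksBP is a spawner actor that periodically throws Blocks actors, apparently as moving scenery for the Void background.
; Tick accumulates delta time and, once it passes CooldownRate, spawns a block at a random point within the central half of the Box component's bounds.
; Each block's static mesh then receives a random physics impulse, driven strongly along negative world Y with slight X and Z jitter.
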(event `self.ReceiveTick`
  (params (DeltaSeconds :type "Float (single-precision)"))
  (bind (_origin _boxextent) (`KismetSystemLibrary.GetComponentBounds` (`self.Box`)))
  (bind _returnvalue (/ (.z _boxextent) 2.0))
  (bind _returnvalue_2 (/ (.x _boxextent) 2.0))
  (bind _returnvalue_3 (/ (.y _boxextent) 2.0))
  (bind _output_get (set `self.SpawnBlockCool` (+ DeltaSeconds (`self.SpawnBlockCool`))))
  (if (> _output_get (`self.CooldownRate`))
    (set `self.SpawnBlockCool` 0.0)
    (bind _returnvalue_4 (`|SpawnActorFromClass` "/Game/Enviroment/Void/Background/Blocks.Blocks_C" (`KismetMathLibrary.MakeTransform` (+ (`KismetMathLibrary.MakeVector` (`KismetMathLibrary.RandomFloatInRange` (* _returnvalue_2 -1.0) _returnvalue_2) (`KismetMathLibrary.RandomFloatInRange` (* _returnvalue_3 -1.0) _returnvalue_3) (`KismetMathLibrary.RandomFloatInRange` (* _returnvalue -1.0) _returnvalue)) _origin)) "AdjustIfPossibleButAlwaysSpawn" "OverrideRootScale" null null))
    (`PrimitiveComponent.AddImpulse` (`/Game/Enviroment/Void/Background/Blocks.StaticMesh` _returnvalue_4) (* (`KismetMathLibrary.MakeVector` (`KismetMathLibrary.RandomFloatInRange` -10.0 10.0) (`KismetMathLibrary.RandomFloatInRange` -5000.0 -100.0) (`KismetMathLibrary.RandomFloatInRange` -10.0 10.0)) 50) "None" false)))

(fn `UserConstructionScript`)